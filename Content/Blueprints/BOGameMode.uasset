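; Game mode for a block-breaking ball game that tracks score, lives and the win and loss states.
; BeginPlay creates the HUD and resets the game; score and life events then push values to it.
; A lost ball costs points, with score floored at zero, and a life or ends the game.
; Clearing all "block"-tagged actors or game over plays a sound, then opens Level1 after a delay.
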(event Custom|Reset
  (bind _maxlives (Variables|Default|GetMaxLives))
  (bind _hud (Variables|Default|GetHUD))
  ;[1 1 1] Reset Game
  (Variables|Default|SetLives _maxlives)
  (Variables|/Game/Blueprints/BP_HUD.BP_HUD_C|SetLives _hud _maxlives)
  (Variables|/Game/Blueprints/BP_HUD.BP_HUD_C|SetPoints _hud 0)
  (Variables|Default|SetCurrentsPoints 0)
  (Variables|Default|SetGameOver? false))

(event Custom|UpdatePoints
  (params (Points :type Integer))
  ;[1 1 1] Update Score
  (if (<= (+ Points (Variables|Default|GetCurrentsPoints)) 0)
    (Variables|Default|SetCurrentsPoints 0)
    (else
      (Variables|Default|SetCurrentsPoints (+ Points (Variables|Default|GetCurrentsPoints)))))
  (Variables|/Game/Blueprints/BP_HUD.BP_HUD_C|SetPoints (Variables|Default|GetHUD) (Variables|Default|GetCurrentsPoints)))

(event Custom|LifeLost
  ;[1 1 1] Losing a Ball
  (CallFunction|UpdatePoints -500)
  (if (<= (Variables|Default|GetLives) 0)
    (CallFunction|GameOver)
    (else
      (bind _output_get (Variables|Default|SetLives (- (Variables|Default|GetLives) 1)))
      (Variables|/Game/Blueprints/BP_HUD.BP_HUD_C|SetLives (Variables|Default|GetHUD) _output_get))))

(event Custom|GameOver
  ;[1 1 1] Game Over
  (Variables|Default|SetGameOver? true)
  (Audio|PlaySound2D "/Game/Audio/GameOver.GameOver" 1.0 1.0 0.0 0 0)
  (Utilities|FlowControl|Delay 5.0)
  (Game|OpenLevel(byName) "Level1"))

(event Custom|Blocks%20Remaining%20Check
  ;[1 1 1] Count Number OF Blocks Left
  (bind _outactors (Actor|GetAllActorswithTag "block"))
  (bind _output_get (Variables|Default|SetBlocksRemaining (Utilities|Array|Length _outactors)))
  (if (<= _output_get 0)
    (CallFunction|LevelClear)))

(event Custom|Level%20Clear
  ;[1 1 1] Check if Level Clear
  (Variables|Default|SetLevelClear? true)
  (Audio|PlaySound2D "/Game/Audio/LevelClear.LevelClear" 1.0 1.0 0.0 0 0)
  (Utilities|FlowControl|Delay 5.0)
  (Game|OpenLevel(byName) "Level1"))

(event EventBeginPlay
  ;[1 1 1] Add HUD
  (bind _returnvalue (UserInterface|CreateWidget "/Game/Blueprints/BP_HUD.BP_HUD_C"))
  (bind _output_get (Variables|Default|SetHUD _returnvalue))
  (UserInterface|Viewport|AddtoViewport _output_get 0)
  (CallFunction|Reset))

(fn ConstructionScript)