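; Block tower actor with a destructible component that crumbles and removes itself when fractured.
; On fracture it enables gravity and sets the debris to ignore physics bodies while blocking other destructibles and static world geometry.
; A radial impulse from just above the component's location pushes the pieces, a crumble sound plays in 2D, and the actor is destroyed after a short delay.
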(event OnComponentFracture(Destructible)
  (params (HitPoint :type Vector%20%28by%20ref%29 :default "0, 0, 0") (HitDirection :type Vector%20%28by%20ref%29 :default "0, 0, 0"))
  (bind _destructible (Variables|Default|GetDestructible))
  (bind _returnvalue (Transformation|GetWorldLocation _destructible))
  (Physics|SetEnableGravity (Variables|Default|GetDestructible) true)
  (Collision|SetCollisionResponsetoChannel (Variables|Default|GetDestructible) "ECC_PhysicsBody" "ECR_Ignore")
  (Collision|SetCollisionResponsetoChannel (Variables|Default|GetDestructible) "ECC_Destructible" "ECR_Block")
  (Collision|SetCollisionResponsetoChannel (Variables|Default|GetDestructible) "ECC_WorldStatic" "ECR_Block")
  (Physics|AddRadialImpulse _destructible (Math|Vector|MakeVector (.x _returnvalue) (.y _returnvalue) (+ (.z _returnvalue) 5e+01)) 4e+01 5e+03 "RIF_Constant" false)
  (Audio|PlaySound2D "/Game/Audio/Crumble.Crumble" 1.0 1.0 0.0 0 0)
  (Utilities|FlowControl|Delay 1.5)
  (Actor|DestroyActor))

(fn ConstructionScript)