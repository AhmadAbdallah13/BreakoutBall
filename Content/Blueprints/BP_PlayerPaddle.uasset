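; Player paddle for a ball-and-paddle game that spawns, launches and steers play of the ball.
; It caches the BOGameMode on BeginPlay and spawns a BP_Ball at its Arrow unless the game is over.
; Axis input pushes the paddle with physics impulses, while touch sets its clamped X position from the deprojected screen point.
; FireBall or a flick gesture launches an inactive ball, and ball hits play a sound.
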(event OnComponentHit(Paddle)
  (params (HitComponent :type Primitive%20Component%20Object%20Reference) (OtherActor :type Actor%20Object%20Reference) (OtherComp :type Primitive%20Component%20Object%20Reference) (NormalImpulse :type Vector :default "0, 0, 0") (Hit :type Hit%20Result%20Structure%20%28by%20ref%29))
  ;[1 1 1] Play Sound
  (Utilities|Casting|CastToBP_Ball OtherActor)
  (Audio|PlaySound2D "/Game/Audio/Hit.Hit" 1.0 1.0 0.0 0 0))

(event Custom|SpawnNewBall
  ;[1 1 1] Spawn Ball
  (if (not (Variables|/Game/Blueprints/BOGameMode.BOGameMode_C|GetGameOver? (Variables|Default|GetGameMode)))
    (bind _returnvalue (Game|SpawnActorfromClass "/Game/Blueprints/BP_Ball.BP_Ball_C" (Transformation|GetWorldTransform (Variables|Default|GetArrow)) "Undefined" 0 0))
    (Variables|Default|SetBall _returnvalue)))

(event EventBeginPlay
  ;[1 1 1] Get GameMode
  (bind _asbogame_mode (Utilities|Casting|CastToBOGameMode (Game|GetGameMode)))
  (Variables|Default|SetGameMode _asbogame_mode)
  (CallFunction|SpawnNewBall))

(event Input|ActionEvents|InputActionFireBall
  (params (Key :type Key%20Structure :default "None"))
  (bind _ball (Variables|Default|GetBall))
  (:Pressed
    ;[1 1 1] FireBall
    (if (and (Utilities|IsValid _ball) (not (Variables|/Game/Blueprints/BP_Ball.BP_Ball_C|GetActive _ball)))
      (Default|LaunchBall (Variables|Default|GetBall)))))

(event Input|AxisEvents|InputAxisHorizontalMovement
  (params (AxisValue :type Float%20%28single-precision%29))
  ;[1 1 1] Paddle Movement
  (Physics|AddImpulse (Variables|Default|GetPaddle) (Math|Vector|MakeVector (* AxisValue (Variables|Default|GetSpeed)) 0.0 0.0) "None" false))

(event Input|KeyboardEvents|GestureFlick
  (params (Key :type Key%20Structure :default "None"))
  (bind _ball (Variables|Default|GetBall))
  (:Pressed
    ;[1 1 1] FireBall
    (if (and (Utilities|IsValid _ball) (not (Variables|/Game/Blueprints/BP_Ball.BP_Ball_C|GetActive _ball)))
      (Default|LaunchBall (Variables|Default|GetBall)))))

(event Input|TouchEvents|InputTouch
  (params (Location :type Vector) (FingerIndex :type ETouchIndex%20Enum))
  ;[1 1 1] Touch Control!! FREEZ
  (:Pressed
    (Transformation|SetWorldLocation (Variables|Default|GetPaddle) (Math|Vector|MakeVector (Math|Float|Clamp(Float) (* (.x (.WorldLocation (Class|PlayerController|DeprojectScreenPositiontoWorld (Game|GetPlayerController 0) (.x Location) 0.0))) 1.4e+02) -5.8e+02 602.0) -5e+01 2e+01) false false :!label _label))
  (:Released
    (goto _label))
  (:Moved
    (goto _label)))

(fn ConstructionScript)